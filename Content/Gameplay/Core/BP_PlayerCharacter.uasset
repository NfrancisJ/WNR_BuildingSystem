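; BP_PlayerCharacter is the player character, handling movement and look input along with an on-screen reticle.
; Axis inputs move it along the control rotation's forward and right vectors and drive controller yaw and pitch, with pitch inverted.
; On BeginPlay it creates the Reticle widget and adds it to the viewport, and a ReticleVisibility function shows or hides it.
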(event `self.ReceiveBeginPlay`
  (`self.Create HUD`))

(event `InputAxis|Move`
  (params (AxisValue :type "Float (single-precision)"))
  ;[1 1 1] Movement Controls
  (`self.AddMovementInput` (`KismetMathLibrary.GetForwardVector` (`self.GetControlRotation`)) AxisValue))

(event `InputAxis|Straffe`
  (params (AxisValue :type "Float (single-precision)"))
  ;[1 1 1] Movement Controls
  (`self.AddMovementInput` (`KismetMathLibrary.GetRightVector` (`self.GetControlRotation`)) AxisValue))

(event `InputAxis|Yaw`
  (params (AxisValue :type "Float (single-precision)"))
  ;[1 1 1] Movement Controls
  (`self.AddControllerYawInput` AxisValue))

(event `InputAxis|Pitch`
  (params (AxisValue :type "Float (single-precision)"))
  ;[1 1 1] Movement Controls
  (`self.AddControllerPitchInput` (* -1 AxisValue)))

(fn `Create HUD`
  (bind _returnvalue (`|CreateWidget` "/Game/Gameplay/UI/Reticle.Reticle_C"))
  (bind _output_get (set `self.Reticle` _returnvalue))
  (`UserWidget.AddToViewport` _output_get 0))

(fn `ReticleVisibility`
  (params (isVisible :type Boolean))
  (bind _reticle (`self.Reticle`))
  (if isVisible
    (`Widget.SetVisibility` _reticle "Visible")
    (else
      (`Widget.SetVisibility` _reticle "Hidden"))))

(fn `UserConstructionScript`)